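; Lobby actor that moves its camera between a default view and a close-up of a weapon mesh.
; On BeginPlay it stores and prints the camera's starting world transform.
; GoWeaponLoction and RevCamLoc each run a timeline that lerps from the camera's current transform toward an offset weapon view or the stored default.
; A CamMoved flag, updated when each timeline finishes, gates which move can run.
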(event Custom|GoWeaponLoction
  (bind _camera (Variables|Default|GetCamera))
  (if (not (Variables|Default|GetCamMoved))
    (bind _newtrack_0 (Timeline|GoCam Play)
      (:Update
        (Transformation|SetWorldLocation _camera (Math|Vector|Lerp(Vector) (Transformation|GetWorldLocation _camera) (+ (Transformation|GetWorldLocation (Variables|Default|GetWeaponMesh)) "15.000000,-50.000000,50.000000") _newtrack_0) false false)
        (Transformation|SetWorldRotation _camera (Math|Rotator|Lerp(Rotator) (Transformation|GetWorldRotation _camera) (Variables|Default|GetWepRot) _newtrack_0) false false))
      (:Finished
        (Variables|Default|SetCamMoved true)))))

(event Custom|RevCamLoc
  (bind _camera (Variables|Default|GetCamera))
  (bind _camera_2 (Variables|Default|GetCamera))
  (if (Variables|Default|GetCamMoved)
    (bind _newtrack_0 (Timeline|Timeline Play)
      (:Update
        (Transformation|SetWorldLocation _camera_2 (Math|Vector|Lerp(Vector) (Transformation|GetWorldLocation _camera) (Variables|Default|GetCamDefLoc) _newtrack_0) false false)
        (Transformation|SetWorldRotation _camera_2 (Math|Rotator|Lerp(Rotator) (Transformation|GetWorldRotation _camera) (Variables|Default|GetCamDefRot) _newtrack_0) false false))
      (:Finished
        (Variables|Default|SetCamMoved false)))))

(event EventBeginPlay
  (bind _camera (Variables|Default|GetCamera))
  (bind _output_get (Variables|Default|SetCamDefLoc (Transformation|GetWorldLocation _camera)))
  (bind _output_get_2 (Variables|Default|SetCamDefRot (Transformation|GetWorldRotation _camera)))
  (Development|PrintString (Utilities|String|ToString(Vector) _output_get))
  (Development|PrintString (Utilities|String|ToString(Rotator) _output_get_2)))

(event Collision|EventActorBeginOverlap
  (params (OtherActor :type Actor%20Object%20Reference)))

(fn ConstructionScript)